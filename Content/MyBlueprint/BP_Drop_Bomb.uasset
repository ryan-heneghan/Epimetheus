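; BP_Drop_Bomb is a bomb actor that goes off on contact, judging by its name, and damages the player character it hits.
; The Sphere's hit event applies point damage only when the other actor is player 0, using the impact normal impulse as direction.
; It then adds a particle component at the sphere's relative location, destroys the sphere, and destroys the actor after a short delay.
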(event OnComponentHit(Sphere)
  (params (HitComponent :type Primitive%20Component%20Object%20Reference) (OtherActor :type Actor%20Object%20Reference) (OtherComp :type Primitive%20Component%20Object%20Reference) (NormalImpulse :type Vector :default "0, 0, 0") (Hit :type Hit%20Result%20Structure%20%28by%20ref%29))
  (if (== OtherActor (Game|GetPlayerCharacter 0))
    (Game|Damage|ApplyPointDamage OtherActor (Variables|Default|GetDamage) NormalImpulse Hit))
  (AddComponent|AddParticleSystemComponent true (Math|Transform|MakeTransform (Variables|/Script/Engine.SceneComponent|GetRelativeLocation (Variables|Default|GetSphere)) "0, 0, 0" "1.000000,1.000000,1.000000"))
  (Components|DestroyComponent (Variables|Default|GetSphere))
  (Utilities|FlowControl|Delay 0.2)
  (Actor|DestroyActor))

(fn ConstructionScript)