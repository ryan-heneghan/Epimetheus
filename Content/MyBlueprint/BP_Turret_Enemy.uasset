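; BP_Turret_Enemy is an enemy turret actor that damages the player on contact and is destroyed when its health runs out.
; On BeginPlay it passes itself, the player, its head and a raised fire offset to a TurretAI component, which is set up to handle the turret behavior.
; An EnemyHealth component feeds its percentage to the health bar widget on damage, and its death event destroys the actor.
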(event OnEnemyDead(EnemyHealth)
  (params (causer :type Controller%20Object%20Reference))
  (Actor|DestroyActor))

(event OnComponentHit(Box)
  (params (HitComponent :type Primitive%20Component%20Object%20Reference) (OtherActor :type Actor%20Object%20Reference) (OtherComp :type Primitive%20Component%20Object%20Reference) (NormalImpulse :type Vector :default "0, 0, 0") (Hit :type Hit%20Result%20Structure%20%28by%20ref%29))
  ;[1 1 1] Collsion Damage
  (if (== OtherActor (Game|GetPlayerCharacter 0))
    (Game|Damage|ApplyPointDamage 0 2e+01 NormalImpulse Hit 0 self "/Script/Engine.DamageType")))

(event EventBeginPlay
  (bind _turretai (Variables|Default|GetTurretAI))
  (Variables|/Script/Epimetheus.TurretAIComponent|SetTurret _turretai self)
  (Variables|/Script/Epimetheus.TurretAIComponent|SetPlayer _turretai (Game|GetPlayerCharacter 0))
  (Variables|/Script/Epimetheus.TurretAIComponent|SetTurretHead _turretai (Variables|Default|GetHead))
  (Variables|/Script/Epimetheus.TurretAIComponent|SetFirePositionOffset _turretai "0.000000,0.000000,60.000000")
  (bind _aswbp_ai_health_bar (Utilities|Casting|CastToWBP_AI_HealthBar (UserInterface|GetUserWidgetObject (Variables|Default|GetHealthBar))))
  (Variables|Default|SetHealthWidgetRef _aswbp_ai_health_bar))

(event Game|Damage|EventAnyDamage
  (params (Damage :type Float%20%28single-precision%29) (DamageType :type Damage%20Type%20Object%20Reference) (InstigatedBy :type Controller%20Object%20Reference) (DamageCauser :type Actor%20Object%20Reference))
  ;[1 1 1] Applies damage to health bar
  (Variables|/Game/MyBlueprint/WidgetBluePrints/WBP_AI_HealthBar.WBP_AI_HealthBar_C|SetEnemyHealth (Variables|Default|GetHealthWidgetRef) (Variables|/Script/Epimetheus.EnemyHealthComponent|GetCurrentHealthPercent (Variables|Default|GetEnemyHealth))))

(fn ConstructionScript)