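; BP_Bomber_Enemy is an enemy that drops bombs when the player crosses its detection ray.
; A self-repeating Delay loop line-traces along CastPoint's forward vector, rechecking almost every frame and pausing briefly after each drop.
; When the trace hits the player character, it spawns BP_Drop_Bomb at CastPoint's transform.
; Its Cube also deals point damage to whatever it hits, and EnemyHealth receives a self reference on BeginPlay.
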(event OnComponentHit(Cube)
  (params (HitComponent :type Primitive%20Component%20Object%20Reference) (OtherActor :type Actor%20Object%20Reference) (OtherComp :type Primitive%20Component%20Object%20Reference) (NormalImpulse :type Vector :default "0, 0, 0") (Hit :type Hit%20Result%20Structure%20%28by%20ref%29))
  (Game|Damage|ApplyPointDamage OtherActor 1e+01 NormalImpulse Hit))

(event Custom|DropBomb
  (Game|SpawnActorfromClass "/Game/MyBlueprint/BP_Drop_Bomb.BP_Drop_Bomb_C" (Transformation|GetWorldTransform (Variables|Default|GetCastPoint)) "Undefined" 0 0))

(event Custom|CheckWithRay
  (bind _castpoint (Variables|Default|GetCastPoint))
  (bind _returnvalue (Transformation|GetWorldLocation _castpoint))
  ;[1 1 1] Comment
  (bind _outhit (Collision|LineTraceForObjects _returnvalue (+ _returnvalue (* (Math|Vector|GetForwardVector _castpoint) (Variables|Default|GetRayDistance))) (Utilities|Array|MakeArray "ObjectTypeQuery7") false 0 "None"))
  (if (== (.HitActor (Collision|BreakHitResult _outhit)) (Variables|Default|GetPlayerRef))
    (CallFunction|DropBomb)
    (Utilities|FlowControl|Delay 2.0)
    (else
      (Utilities|FlowControl|Delay 0.017)))
  (CallFunction|CheckwithRay))

(event EventBeginPlay
  (Variables|Default|SetPlayerRef (Game|GetPlayerCharacter 0))
  (Variables|/Script/Epimetheus.EnemyHealthComponent|SetEnemySelf (Variables|Default|GetEnemyHealth) self)
  (CallFunction|CheckwithRay))

(fn ConstructionScript)