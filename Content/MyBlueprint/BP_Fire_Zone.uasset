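; BP_Fire_Zone is a hazard volume that deals environmental damage to the player while they stand inside it.
; Box overlap events maintain an InArea flag for player 0's character, and Tick applies a small fixed damage while it is set.
; Damage is frame-rate dependent, as it is not scaled by delta time.
; Any other actor beginning overlap clears the flag, even with the player still inside.
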(event OnComponentBeginOverlap(Box)
  (params (OverlappedComponent :type Primitive%20Component%20Object%20Reference) (OtherActor :type Actor%20Object%20Reference) (OtherComp :type Primitive%20Component%20Object%20Reference) (OtherBodyIndex :type Integer) (bFromSweep :type Boolean) (SweepResult :type Hit%20Result%20Structure%20%28by%20ref%29))
  ;[1 1 1] Check if player is in area
  (Variables|Default|SetInArea (== OtherActor (Game|GetPlayerCharacter 0))))

(event OnComponentEndOverlap(Box)
  (params (OverlappedComponent :type Primitive%20Component%20Object%20Reference) (OtherActor :type Actor%20Object%20Reference) (OtherComp :type Primitive%20Component%20Object%20Reference) (OtherBodyIndex :type Integer))
  ;[1 1 1] Check if player is in area
  (if (== OtherActor (Game|GetPlayerCharacter 0))
    (Variables|Default|SetInArea false)))

(event EventBeginPlay)

(event EventTick
  (params (DeltaSeconds :type Float%20%28single-precision%29))
  (if (Variables|Default|GetInArea)
    (Game|Damage|ApplyDamage (Game|GetPlayerCharacter 0) 0.2 0 self "/Engine/EngineDamageTypes/DmgTypeBP_Environmental.DmgTypeBP_Environmental_C")))

(fn ConstructionScript)