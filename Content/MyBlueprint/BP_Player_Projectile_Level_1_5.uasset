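; BP_Player_Projectile_Level_1_5 is a player projectile that damages the actor it hits.
; A hit on its Sphere component applies the Damage value, adds a particle system component at the sphere's relative transform, and destroys the sphere.
; The actor destroys itself after a short delay following the hit, or when the lifetime timer started on BeginPlay runs out.
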(event OnComponentHit(Sphere)
  (params (HitComponent :type Primitive%20Component%20Object%20Reference) (OtherActor :type Actor%20Object%20Reference) (OtherComp :type Primitive%20Component%20Object%20Reference) (NormalImpulse :type Vector :default "0, 0, 0") (Hit :type Hit%20Result%20Structure%20%28by%20ref%29))
  (Game|Damage|ApplyDamage OtherActor (Variables|Default|GetDamage) 0 0)
  (AddComponent|AddParticleSystemComponent true (Transformation|GetRelativeTransform (Variables|Default|GetSphere)))
  (Components|DestroyComponent (Variables|Default|GetSphere))
  (Utilities|FlowControl|Delay 0.2)
  (Actor|DestroyActor))

(event EventBeginPlay
  (Utilities|FlowControl|Delay 5.0)
  (Actor|DestroyActor))

(fn ConstructionScript)